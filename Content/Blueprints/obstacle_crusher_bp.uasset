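; Obstacle crusher that slides a cube back and forth on a looping timeline, with random pauses at each end.
; CanCrunch turns on at full extension and off once fully retracted.
; Tick checks the player's overlap with a sphere and, once per crunch, deals damage, plays sounds, disables jumping and squashes the player mesh.
; Leaving the sphere restores jumping, then after a short delay reverses the squash and re-arms the hit.
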(event `self.ReceiveBeginPlay`
  (bind _returnvalue (`KismetMathLibrary.RandomFloatInRange` (`self.minDelay`) (`self.maxDelay`)))
  (`TimelineComponent.SetPlayRate` (`self.Timeline_0`) (`self.playRate`))
  (bind (_direction _alpha) (`Timeline|Timeline_0` :!via `PlayFromStart` :!label _label)
    (:`Update`
      (`SceneComponent.K2_SetRelativeLocation` (`self.Cube`) (`KismetMathLibrary.VLerp` (0.0 -250.0 0.0) (0.0 50.0 0.0) _alpha) false false))
    (:`Finished`
      (switch `ETimelineDirection` _direction
        (:`Forward`
          (set `self.canCrunch` true)
          (`KismetSystemLibrary.Delay` _returnvalue)
          (goto _label :!via `ReverseFromEnd`))
        (:`Backward`
          (set `self.canCrunch` false)
          (`KismetSystemLibrary.Delay` _returnvalue)
          (goto _label :!via `PlayFromStart`))))))

(event `self.ReceiveTick`
  (params (DeltaSeconds :type "Float (single-precision)"))
  (bind _returnvalue (`GameplayStatics.GetPlayerCharacter` 0))
  (if (`PrimitiveComponent.IsOverlappingActor` (`self.Sphere`) _returnvalue)
    (bind _asplayer_acorn (cast `/Game/Player/Player_Acorn` _returnvalue))
    (if (`self.canCrunch`)
      (`/Engine/EditorBlueprintResources/StandardMacros.DoOnce` false :!label _label_2
        (:`Completed`
          (`|ExecutionSequence`
            (:`then_0`
              (set `/Game/Player/Player_Acorn.canJump?` false _asplayer_acorn)
              (bind (_direction _alpha) (`Timeline|Timeline_1` :!via `PlayFromStart` :!label _label_3)
                (:`Update`
                  (bind _asplayer_acorn_2 (`/Game/Blueprints/7646_fuctionLibrary.getPlayer`))
                  (`SceneComponent.SetRelativeScale3D` (`Character.Mesh` _asplayer_acorn_2) (`KismetMathLibrary.MakeVector` 0.5 0.5 (`KismetMathLibrary.Lerp` 0.5 0.1 _alpha))))))
            (:`then_1`
              (set `/Game/Player/Player_Acorn.Health` (- (`/Game/Player/Player_Acorn.Health` _asplayer_acorn) 0.2) _asplayer_acorn)
              (`GameplayStatics.PlaySound2D` "/Game/Audio/Sounds/hurt3_Cue.hurt3_Cue" 1.0 1.0 0.0 null null)
              (`GameplayStatics.PlaySound2D` "/Game/Audio/Sounds/kick.kick" 1.0 1.0 0.0 null null)))))
      (else
        (goto _label_2 :!via `Reset`)))))

(event `self.Sphere.OnComponentEndOverlap`
  (params (OverlappedComponent :type "PrimitiveComponent Object Reference") (OtherActor :type "Actor Object Reference") (OtherComp :type "PrimitiveComponent Object Reference") (OtherBodyIndex :type Integer))
  (bind _asplayer_acorn (cast `/Game/Player/Player_Acorn` OtherActor))
  (set `/Game/Player/Player_Acorn.canJump?` true _asplayer_acorn)
  (`KismetSystemLibrary.Delay` 0.5)
  (`|ExecutionSequence`
    (:`then_0`
      (goto _label_2 :!via `Reset`))
    (:`then_1`
      (goto _label_3 :!via `ReverseFromEnd`))))

(fn `UserConstructionScript`)