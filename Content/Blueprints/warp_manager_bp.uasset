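; Warp manager that places the player at a named PlayerStart when play begins.
; On BeginPlay it retries every 0.1 seconds until player character 0 is valid, then moves it to the start the game mode finds using WarpID from acorn_gameInstance.
; A check on the game instance's Warp flag is left unconnected, so the move happens regardless of that flag.
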(event `self.ReceiveBeginPlay`
  (bind _returnvalue (`GameplayStatics.GetPlayerCharacter` 0))
  (`/Engine/EditorBlueprintResources/StandardMacros.IsValid` _returnvalue :!label _label
    (:`Is Valid`
      (`self.K2_SetActorTransform` _returnvalue (`self.GetTransform` (`GameModeBase.K2_FindPlayerStart` (`GameplayStatics.GetGameMode`) null (`KismetStringLibrary.Conv_NameToString` (`/Game/Blueprints/acorn_gameInstance.warpID` (cast `/Game/Blueprints/acorn_gameInstance` (`GameplayStatics.GetGameInstance`) :!pure true))))) false false))
    (:`Is Not Valid`
      (`KismetSystemLibrary.Delay` 0.1)
      (goto _label))))

(fn `UserConstructionScript`)