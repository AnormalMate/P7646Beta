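; Warp entrance trigger that sends the acorn player to another level.
; On box overlap it hides the player, disables movement, stores WarpID and a warp flag in the game instance, and plays a warp sound.
; A forward transition animation runs while all ambient sounds fade out.
; When the animation finishes, it opens the level whose name matches the WarpLevel enum value.
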(event `self.Box.OnComponentBeginOverlap`
  (params (OverlappedComponent :type "PrimitiveComponent Object Reference") (OtherActor :type "Actor Object Reference") (OtherComp :type "PrimitiveComponent Object Reference") (OtherBodyIndex :type Integer) (bFromSweep :type Boolean) (SweepResult :type "HitResult Structure (by ref)"))
  (bind _asplayer_acorn (cast `/Game/Player/Player_Acorn` OtherActor))
  (`self.SetActorHiddenInGame` _asplayer_acorn true)
  (`CharacterMovementComponent.SetMovementMode` (`Character.CharacterMovement` _asplayer_acorn) "MOVE_None" 0)
  (bind _asacorn_game_instance (cast `/Game/Blueprints/acorn_gameInstance` (`GameplayStatics.GetGameInstance`)))
  (set `/Game/Blueprints/acorn_gameInstance.warpID` (`self.warpID`) _asacorn_game_instance)
  (`GameplayStatics.PlaySound2D` "/Game/Audio/Sounds/Levelwarp_Cue.Levelwarp_Cue" 1.0 1.0 0.0 null null)
  (set `/Game/Blueprints/acorn_gameInstance.warp` true _asacorn_game_instance)
  (bind (_anim1 _returnvalue) (`/Game/Blueprints/7646_fuctionLibrary.transition` "Forward"))
  (`UserWidget.BindToAnimationFinished` _returnvalue _anim1 (delegate `finish`))
  (bind _outactors (`GameplayStatics.GetAllActorsOfClass` "/Script/Engine.AmbientSound"))
  (for _array_element _outactors
    (`AudioComponent.FadeOut` (`AmbientSound.AudioComponent` _array_element) 1.0 0.0 "Linear")))

(event `finish`
  (`GameplayStatics.OpenLevel` (`KismetStringLibrary.Conv_StringToName` (`|GetEnumeratorNameAsString` (`self.warpLevel`))) (`self.SaveSettings`)))

(fn `UserConstructionScript`)