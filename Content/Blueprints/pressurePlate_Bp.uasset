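; Pressure plate switch that Player_Acorn turns on by overlapping its Box.
; It works as a latch, a toggle when FlipFlop is set, or, when Timed takes priority, switches off after a delay.
; Tick watches IsOn through two DoOnce gates that reset each other, so each state change snaps Cube1 down or up and plays SwitchCue once.
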(event `self.ReceiveTick`
  (params (DeltaSeconds :type "Float (single-precision)"))
  (bind _cube1 (`self.Cube1`))
  (bind _switch_cue (`self.switch_Cue`))
  (if (`self.isOn`)
    (`/Engine/EditorBlueprintResources/StandardMacros.DoOnce` false :!label _label
      (:`Completed`
        (`SceneComponent.K2_SetRelativeLocation` _cube1 (0.0 0.0 5.0) false false)
        (`AudioComponent.Play` _switch_cue 0.0)
        (goto _label_2 :!via `Reset`)))
    (else
      (`/Engine/EditorBlueprintResources/StandardMacros.DoOnce` false :!label _label_2
        (:`Completed`
          (`SceneComponent.K2_SetRelativeLocation` _cube1 (0.0 0.0 20.0) false false)
          (`AudioComponent.Play` _switch_cue 0.0)
          (goto _label :!via `Reset`))))))

(event `self.Box.OnComponentBeginOverlap`
  (params (OverlappedComponent :type "PrimitiveComponent Object Reference") (OtherActor :type "Actor Object Reference") (OtherComp :type "PrimitiveComponent Object Reference") (OtherBodyIndex :type Integer) (bFromSweep :type Boolean) (SweepResult :type "HitResult Structure (by ref)"))
  (cast `/Game/Player/Player_Acorn` OtherActor)
  (if (`self.timed`)
    (if (not (`self.isOn`))
      (set `self.isOn` true)
      (`|ExecutionSequence`
        (:`then_0`
          (`KismetSystemLibrary.Delay` (`self.time`))
          (set `self.isOn` false))))
    (elif (`self.flipFlop`)
      (set `self.isOn` (not (`self.isOn`)))
      (else
        (set `self.isOn` true)))))

(fn `UserConstructionScript`)