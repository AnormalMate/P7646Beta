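; A platform Blueprint that sinks when the Player_Acorn character enters its Box trigger.
; After a short delay, MoveComponentTo eases the Cube vertically to ZLoc over the Speed duration, keeping its X and Y.
; Following a longer wait, it eases the Cube back to a relative Z left at the pin's default, over the same duration.
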(event `self.Box.OnComponentBeginOverlap`
  (params (OverlappedComponent :type "PrimitiveComponent Object Reference") (OtherActor :type "Actor Object Reference") (OtherComp :type "PrimitiveComponent Object Reference") (OtherBodyIndex :type Integer) (bFromSweep :type Boolean) (SweepResult :type "HitResult Structure (by ref)"))
  (bind _cube (`self.Cube`))
  (bind (_relativelocation_x _relativelocation_y) (`KismetMathLibrary.BreakVector` (`SceneComponent.RelativeLocation` _cube)))
  (cast `/Game/Player/Player_Acorn` OtherActor)
  (`KismetSystemLibrary.Delay` 0.2)
  (`KismetSystemLibrary.MoveComponentTo` _cube (`KismetMathLibrary.MakeVector` _relativelocation_x _relativelocation_y (`self.zLoc`)) (struct) true true (`self.speed`))
  (`KismetSystemLibrary.Delay` 7.0)
  (`KismetSystemLibrary.MoveComponentTo` (`self.Cube`) (`KismetMathLibrary.MakeVector` _relativelocation_x _relativelocation_y) (struct) true true (`self.speed`)))

(fn `UserConstructionScript`)