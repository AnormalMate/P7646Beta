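; Obstacle pusher that slides a cube back and forth and launches the player acorn out of its push area.
; A timeline lerps the cube along its local Y axis, reversing after a random delay at each end.
; Tick polls the push area and launches Player_Acorn along the arrow's forward vector with a slight lift.
; A DoOnce limits this to one launch per overlap, independent of the timeline's state.
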(event `self.ReceiveBeginPlay`
  (bind _returnvalue (`KismetMathLibrary.RandomFloatInRange` (`self.mindelay`) (`self.maxdelay`)))
  (`TimelineComponent.SetPlayRate` (`self.Timeline_0`) (`self.playRate`))
  (bind (_direction _alpha) (`Timeline|Timeline_0` :!via `PlayFromStart` :!label _label)
    (:`Update`
      (`SceneComponent.K2_SetRelativeLocation` (`self.Cube`) (`KismetMathLibrary.VLerp` (0.0 -250.0 0.0) (0.0 50.0 0.0) _alpha) false false))
    (:`Finished`
      (switch `ETimelineDirection` _direction
        (:`Forward`
          (`KismetSystemLibrary.Delay` _returnvalue)
          (goto _label :!via `ReverseFromEnd`))
        (:`Backward`
          (`KismetSystemLibrary.Delay` _returnvalue)
          (goto _label :!via `PlayFromStart`))))))

(event `self.ReceiveTick`
  (params (DeltaSeconds :type "Float (single-precision)"))
  (bind _returnvalue (`GameplayStatics.GetPlayerCharacter` 0))
  (bind (_returnvalue_x _returnvalue_y) (`KismetMathLibrary.BreakVector` (* (`SceneComponent.GetForwardVector` (`self.Arrow`)) (`self.pushSpeed`))))
  (if (`PrimitiveComponent.IsOverlappingActor` (`self.pushArea`) _returnvalue)
    (`/Engine/EditorBlueprintResources/StandardMacros.DoOnce` false :!label _label_2
      (:`Completed`
        (bind _asplayer_acorn (cast `/Game/Player/Player_Acorn` _returnvalue))
        (`Character.LaunchCharacter` _asplayer_acorn (`KismetMathLibrary.MakeVector` _returnvalue_x _returnvalue_y 100.0) true true)))
    (else
      (goto _label_2 :!via `Reset`))))

(fn `UserConstructionScript`)