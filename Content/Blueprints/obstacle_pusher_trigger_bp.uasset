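; Pusher obstacle that shoves a cube outward when the player enters its trigger and launches Player_Acorn.
; Tick polls both overlaps: Trigger starts a DoOnce-gated timeline that slides the cube, waits a random delay, then reverses and re-arms.
; PushArea launches the player along the Arrow with a fixed lift if Canpush is set during the stroke, checking only once per overlap.
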(event `self.ReceiveTick`
  (params (DeltaSeconds :type "Float (single-precision)"))
  (bind _returnvalue (`GameplayStatics.GetPlayerCharacter` 0))
  (bind (_returnvalue_x _returnvalue_y) (`KismetMathLibrary.BreakVector` (* (`SceneComponent.GetForwardVector` (`self.Arrow`)) (`self.pushSpeed`))))
  (`|ExecutionSequence`
    (:`then_0`
      (if (`PrimitiveComponent.IsOverlappingActor` (`self.trigger`) _returnvalue)
        (`/Engine/EditorBlueprintResources/StandardMacros.DoOnce` false :!label _label
          (:`Completed`
            (`TimelineComponent.SetPlayRate` (`self.Timeline_0`) (`self.playRate`))
            (bind (_direction _alpha) (`Timeline|Timeline_0` :!via `PlayFromStart` :!label _label_2)
              (:`Update`
                (`SceneComponent.K2_SetRelativeLocation` (`self.Cube`) (`KismetMathLibrary.VLerp` (0.0 -250.0 0.0) (0.0 50.0 0.0) _alpha) false false)
                (set `self.canpush` true))
              (:`Finished`
                (switch `ETimelineDirection` _direction
                  (:`Forward`
                    (set `self.canpush` false)
                    (`KismetSystemLibrary.Delay` (`KismetMathLibrary.RandomFloatInRange` (`self.mindelay`) (`self.maxdelay`)))
                    (goto _label_2 :!via `ReverseFromEnd`))
                  (:`Backward`
                    (goto _label :!via `Reset`)))))))))
    (:`then_1`
      (if (`PrimitiveComponent.IsOverlappingActor` (`self.pushArea`) _returnvalue)
        (`/Engine/EditorBlueprintResources/StandardMacros.DoOnce` false :!label _label_3
          (:`Completed`
            (if (`self.canpush`)
              (bind _asplayer_acorn (cast `/Game/Player/Player_Acorn` _returnvalue))
              (`Character.LaunchCharacter` _asplayer_acorn (`KismetMathLibrary.MakeVector` _returnvalue_x _returnvalue_y 100.0) true true))))
        (else
          (goto _label_3 :!via `Reset`))))))

(fn `UserConstructionScript`)