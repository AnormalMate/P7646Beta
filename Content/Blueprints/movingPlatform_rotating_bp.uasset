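; Rotating moving-platform actor that spins continuously about its local X (roll) axis.
; On BeginPlay, a looping 0.01-second timer calls the rotatePlatform event instead of using Tick.
; Each call adds RotationSpeed as a local roll delta to DefaultSceneRoot, so the value acts as degrees per timer call rather than per second.
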(event `self.ReceiveBeginPlay`
  (`parent.ReceiveBeginPlay`)
  (`KismetSystemLibrary.K2_SetTimerDelegate` (delegate `rotatePlatform`) 0.01 true))

(event `rotatePlatform`
  (`SceneComponent.K2_AddLocalRotation` (`self.DefaultSceneRoot`) (`KismetMathLibrary.MakeRotator` (`self.rotationSpeed`)) false false))

(fn `UserConstructionScript`
  (`parent.UserConstructionScript`))