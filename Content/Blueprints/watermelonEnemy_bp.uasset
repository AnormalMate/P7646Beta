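; Watermelon enemy that rolls around the level, chases the acorn player on sight and squashes them on contact.
; It wanders to random navigable points and chases inside SightRange, moving by capsule forces while a timeline spins its face during chases.
; Contact disables jumping, flattens the player's mesh, deals damage and swaps the capsule's collision type until shortly after separation.
; Punch launches it along the player's forward vector and briefly shows a kicked face.
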(event `wander`
  (bind _returnvalue (`self.K2_GetActorLocation`))
  (bind (_returnvalue_roll _returnvalue_pitch) (`KismetMathLibrary.BreakRotator` (`self.K2_GetActorRotation`)))
  (bind (_returnvalue_x _returnvalue_y) (`KismetMathLibrary.BreakVector` (* (`self.GetActorForwardVector`) 2000)))
  (bind (_returnvalue_roll_2 _returnvalue_pitch_2 _returnvalue_yaw) (`KismetMathLibrary.BreakRotator` (`KismetMathLibrary.FindLookAtRotation` _returnvalue (`self.locationToMove`))))
  (`SceneComponent.K2_SetRelativeRotation` :`self` (`self.faceParent`))
  (if (not (`self.chase?`))
    (set `self.locationToMove` (`NavigationSystemV1.K2_GetRandomLocationInNavigableRadius` _returnvalue 4000.0 null null))
    (`self.K2_SetActorRotation` (`KismetMathLibrary.MakeRotator` 0.0 _returnvalue_pitch _returnvalue_yaw) :!label _label)
    (if (not (`self.chase?`))
      (`PrimitiveComponent.AddForce` (`self.CapsuleComponent`) (`KismetMathLibrary.MakeVector` _returnvalue_x _returnvalue_y) "None" true)
      (`KismetSystemLibrary.Delay` 0.01)
      (if (== (`self.locationToMove`) (`self.K2_GetActorLocation`) :`ErrorTolerance` 1000.0)
        (`self.wander`)
        (else
          (goto _label))))))

(event `self.ReceiveBeginPlay`
  (`self.wander`))

(event `self.ReceiveTick`
  (params (DeltaSeconds :type "Float (single-precision)"))
  (bind _returnvalue (`GameplayStatics.GetPlayerCharacter` 0))
  (bind (_returnvalue_x _returnvalue_y) (`KismetMathLibrary.BreakVector` (* (`self.GetActorForwardVector`) 1000)))
  (bind (_returnvalue_roll _returnvalue_pitch _returnvalue_yaw) (`KismetMathLibrary.BreakRotator` (`KismetMathLibrary.FindLookAtRotation` (`self.K2_GetActorLocation`) (`self.K2_GetActorLocation` _returnvalue))))
  (`|ExecutionSequence`
    (:`then_0`
      (if (`self.chase?`)
        (`/Engine/EditorBlueprintResources/StandardMacros.DoOnce` false :!label _label_2
          (:`Completed`
            (bind (_direction _alpha) (`Timeline|Timeline_0` :!via `PlayFromStart`)
              (:`Update`
                (`SceneComponent.K2_SetRelativeRotation` (`self.faceParent`) (`KismetMathLibrary.MakeRotator` 0.0 (`KismetMathLibrary.Lerp` 0.0 -360.0 _alpha)) false false))
              (:`Finished`
                (goto _label_2 :!via `Reset`)))))))
    (:`then_1`
      (if (`PrimitiveComponent.IsOverlappingActor` (`self.sightRange`) _returnvalue)
        (set `self.chase?` true)
        (`self.K2_SetActorRotation` (`KismetMathLibrary.MakeRotator` 0.0 0.0 _returnvalue_yaw))
        (`PrimitiveComponent.AddForce` (`self.CapsuleComponent`) (`KismetMathLibrary.MakeVector` _returnvalue_x _returnvalue_y) "None" true)))))

(event `self.sightRange.OnComponentEndOverlap`
  (params (OverlappedComponent :type "PrimitiveComponent Object Reference") (OtherActor :type "Actor Object Reference") (OtherComp :type "PrimitiveComponent Object Reference") (OtherBodyIndex :type Integer))
  (cast `/Game/Player/Player_Acorn` OtherActor)
  (set `self.chase?` false)
  (`self.wander`))

(event `self.Sphere.OnComponentBeginOverlap`
  (params (OverlappedComponent :type "PrimitiveComponent Object Reference") (OtherActor :type "Actor Object Reference") (OtherComp :type "PrimitiveComponent Object Reference") (OtherBodyIndex :type Integer) (bFromSweep :type Boolean) (SweepResult :type "HitResult Structure (by ref)"))
  (bind _asplayer_acorn (cast `/Game/Player/Player_Acorn` OtherActor))
  (`PrimitiveComponent.SetCollisionObjectType` (`self.CapsuleComponent`) "ECC_Vehicle")
  (`|ExecutionSequence`
    (:`then_0`
      (set `/Game/Player/Player_Acorn.canJump?` false _asplayer_acorn)
      (bind (_direction _alpha) (`Timeline|Timeline_1` :!via `PlayFromStart` :!label _label_3)
        (:`Update`
          (bind _asplayer_acorn_2 (`/Game/Blueprints/7646_fuctionLibrary.getPlayer`))
          (`SceneComponent.SetRelativeScale3D` (`Character.Mesh` _asplayer_acorn_2) (`KismetMathLibrary.MakeVector` 0.5 0.5 (`KismetMathLibrary.Lerp` 0.5 0.1 _alpha))))))
    (:`then_1`
      (set `/Game/Player/Player_Acorn.Health` (- (`/Game/Player/Player_Acorn.Health` _asplayer_acorn) 0.2) _asplayer_acorn)
      (`GameplayStatics.PlaySound2D` "/Game/Audio/Sounds/hurt3_Cue.hurt3_Cue" 1.0 1.0 0.0 null null))))

(event `self.Sphere.OnComponentEndOverlap`
  (params (OverlappedComponent :type "PrimitiveComponent Object Reference") (OtherActor :type "Actor Object Reference") (OtherComp :type "PrimitiveComponent Object Reference") (OtherBodyIndex :type Integer))
  (bind _asplayer_acorn (cast `/Game/Player/Player_Acorn` OtherActor))
  (set `/Game/Player/Player_Acorn.canJump?` true _asplayer_acorn)
  (`KismetSystemLibrary.Delay` 0.5)
  (`PrimitiveComponent.SetCollisionObjectType` (`self.CapsuleComponent`) "ECC_Pawn")
  (goto _label_3 :!via `ReverseFromEnd`))

(event `/Game/Blueprints/7646_blueprintInterface.punch`
  (bind _asplayer_acorn (`/Game/Blueprints/7646_fuctionLibrary.getPlayer`))
  (bind (_returnvalue_x _returnvalue_y) (`KismetMathLibrary.BreakVector` (* (`self.GetActorForwardVector` _asplayer_acorn) 50000.0)))
  (`PrimitiveComponent.AddForce` (`self.CapsuleComponent`) (`KismetMathLibrary.MakeVector` _returnvalue_x _returnvalue_y 1000.0) "None" true)
  (`PrimitiveComponent.SetMaterial` (`self.face`) 0 "/Game/Materials/watermelonFaceKicked_m.watermelonFaceKicked_m")
  (`KismetSystemLibrary.Delay` 1.0)
  (`PrimitiveComponent.SetMaterial` (`self.face`) 0 "/Game/Materials/watermelonFace_m.watermelonFace_m"))

(fn `UserConstructionScript`)