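; Red apple enemy that wanders random navigable points and chases Player_Acorn.
; A detection sphere starts the AIMoveTo chase; leaving it or failing the move resumes wandering after a delay.
; The Attack overlap, gated by a DoOnce that resets shortly after exit, damages and knocks back a living player, then resumes chasing.
; Punch disables attacking, pops the apple upward, plays its death animation and destroys it.
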(event `wander`
  (if (not (`self.chase`))
    (`|AIMoveTo` self (`NavigationSystemV1.K2_GetRandomLocationInNavigableRadius` (`self.K2_GetActorLocation`) 1000.0 null null) null
      (:`OnSuccess`
        _)
      (:`OnFail`
        _))
    (`self.wander`)))

(event `self.ReceiveBeginPlay`
  (`self.wander`))

(event `chasePlayer`
  (if (`self.chase`)
    (`|AIMoveTo` self (0.0 0.0 0.0) (stale `self.Sphere.OnComponentBeginOverlap` _asplayer_acorn) :!label _label
      (:`OnFail`
        (`KismetSystemLibrary.Delay` 3.0 :!label _label_2)
        (set `self.chase` false)
        (`self.wander`)))))

(event `self.Sphere.OnComponentBeginOverlap`
  (params (OverlappedComponent :type "PrimitiveComponent Object Reference") (OtherActor :type "Actor Object Reference") (OtherComp :type "PrimitiveComponent Object Reference") (OtherBodyIndex :type Integer) (bFromSweep :type Boolean) (SweepResult :type "HitResult Structure (by ref)"))
  (bind _asplayer_acorn (cast `/Game/Player/Player_Acorn` OtherActor))
  (set `self.chase` true)
  (goto _label))

(event `self.Sphere.OnComponentEndOverlap`
  (params (OverlappedComponent :type "PrimitiveComponent Object Reference") (OtherActor :type "Actor Object Reference") (OtherComp :type "PrimitiveComponent Object Reference") (OtherBodyIndex :type Integer))
  (cast `/Game/Player/Player_Acorn` OtherActor)
  (goto _label_2))

(event `self.attack.OnComponentBeginOverlap`
  (params (OverlappedComponent :type "PrimitiveComponent Object Reference") (OtherActor :type "Actor Object Reference") (OtherComp :type "PrimitiveComponent Object Reference") (OtherBodyIndex :type Integer) (bFromSweep :type Boolean) (SweepResult :type "HitResult Structure (by ref)"))
  (bind _mesh (`self.Mesh`))
  (bind _asplayer_acorn (cast `/Game/Player/Player_Acorn` OtherActor))
  (if (not (`/Game/Player/Player_Acorn.dead?` _asplayer_acorn))
    (`/Engine/EditorBlueprintResources/StandardMacros.DoOnce` false :!label _label_3
      (:`Completed`
        (if (`self.canAttack?`)
          (set `/Game/Player/Player_Acorn.Health` (- (`/Game/Player/Player_Acorn.Health` _asplayer_acorn) 0.2) _asplayer_acorn)
          (`GameplayStatics.PlaySound2D` "/Game/Audio/Sounds/hurt3_Cue.hurt3_Cue" 1.0 1.0 0.0 null null)
          (bind (_returnvalue_x _returnvalue_y) (`KismetMathLibrary.BreakVector` (* (`self.GetActorForwardVector` _asplayer_acorn) -500)))
          (`self.LaunchCharacter` _asplayer_acorn (`KismetMathLibrary.MakeVector` _returnvalue_x _returnvalue_y 500.0) true true)
          (bind _returnvalue (`/Game/Blueprints/7646_fuctionLibrary.playAnimationLength` _mesh "/Game/Character/RedApple_anims_Armature_attack.RedApple_anims_Armature_attack"))
          (`KismetSystemLibrary.Delay` _returnvalue)
          (`SkeletalMeshComponent.PlayAnimation` _mesh "/Game/Character/RedApple_anims_Armature_walk.RedApple_anims_Armature_walk" true)
          (`self.chasePlayer`))))))

(event `self.attack.OnComponentEndOverlap`
  (params (OverlappedComponent :type "PrimitiveComponent Object Reference") (OtherActor :type "Actor Object Reference") (OtherComp :type "PrimitiveComponent Object Reference") (OtherBodyIndex :type Integer))
  (cast `/Game/Player/Player_Acorn` OtherActor)
  (`KismetSystemLibrary.Delay` 1.0)
  (goto _label_3 :!via `Reset`))

(event `/Game/Blueprints/7646_blueprintInterface.punch`
  (`/Game/Blueprints/7646_fuctionLibrary.getPlayer`)
  (set `self.canAttack?` false)
  (`self.LaunchCharacter` (0.0 0.0 500.0) true true)
  (bind _returnvalue (`/Game/Blueprints/7646_fuctionLibrary.playAnimationLength` (`self.Mesh`) "/Game/Character/RedApple_anims_Armature_die.RedApple_anims_Armature_die"))
  (`KismetSystemLibrary.Delay` _returnvalue)
  (`KismetSystemLibrary.Delay` 0.5)
  (`self.K2_DestroyActor`))

(fn `UserConstructionScript`)