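; Level goal pickup that ends the level when Player_Acorn touches it and returns to the Lobby.
; On BeginPlay it polls for the save slot, then shows a completed sprite if its ID is in the saved GoalsID.
; On overlap it disables input, hides the billboard and stops the player with a slight upward launch.
; First-time collection increments goal counts, records the ID, plays the UI animation and saves.
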(event `self.ReceiveBeginPlay`
  (bind (_save _returnvalue) (`/Game/Blueprints/7646_fuctionLibrary.getSaveSlot`))
  (`KismetSystemLibrary.Delay` 0.1)
  (bind _returnvalue_2 (`GameplayStatics.DoesSaveGameExist` _returnvalue :!label _label))
  (if _returnvalue_2
    (bind _returnvalue_3 (`GameplayStatics.LoadGameFromSlot` _returnvalue))
    (bind _asdefault_save_game (cast `/Game/Blueprints/defaultSaveGame` _returnvalue_3))
    (bind _output_get (set `self.save` _asdefault_save_game))
    (`KismetSystemLibrary.Delay` 0.1)
    (for _array_element (`/Game/Blueprints/defaultSaveGame.goalsID` _output_get)
      (if (`KismetStringLibrary.EqualEqual_StrStr` _array_element (`self.ID`))
        (`BillboardComponent.SetSprite` (`self.Billboard`) "/Game/Textures/goal_placeholderCompleted.goal_placeholderCompleted")))
    (else
      (`KismetSystemLibrary.Delay` 0.5)
      (goto _label))))

(event `self.Sphere.OnComponentBeginOverlap`
  (params (OverlappedComponent :type "PrimitiveComponent Object Reference") (OtherActor :type "Actor Object Reference") (OtherComp :type "PrimitiveComponent Object Reference") (OtherBodyIndex :type Integer) (bFromSweep :type Boolean) (SweepResult :type "HitResult Structure (by ref)"))
  (bind (_save _returnvalue) (`/Game/Blueprints/7646_fuctionLibrary.getSaveSlot`))
  (bind (_save_2 _returnvalue_2) (`/Game/Blueprints/7646_fuctionLibrary.getSaveSlot`))
  (bind _asplayer_acorn (cast `/Game/Player/Player_Acorn` OtherActor))
  (`self.DisableInput` _asplayer_acorn (`GameplayStatics.GetPlayerController` 0))
  (`|ExecutionSequence`
    (:`then_0`
      (`SceneComponent.SetHiddenInGame` (`self.Billboard`) true false)
      (if (not (== (`BillboardComponent.Sprite` (`self.Billboard`)) "/Game/Textures/goal_placeholderCompleted.goal_placeholderCompleted"))
        (bind _asplayer_acorn_2 (`/Game/Blueprints/7646_fuctionLibrary.getPlayer`))
        (`/Engine/EditorBlueprintResources/StandardMacros.IncrementInt` (`/Game/Player/Player_Acorn.goals` _asplayer_acorn_2)
          (:`  `
            (bind _save_3 (`/Game/Player/Player_Acorn.save` _asplayer_acorn_2))
            (`/Engine/EditorBlueprintResources/StandardMacros.IncrementInt` (`/Game/Blueprints/defaultSaveGame.goals` _save_3)
              (:`  `
                (`KismetArrayLibrary.Array_Add` (`/Game/Blueprints/defaultSaveGame.goalsID` _save_3) (`self.ID`))
                (`/Game/UI/MainUI2.goalAnimation` (`/Game/Player/Player_Acorn.ui1` _asplayer_acorn))
                (`GameplayStatics.SaveGameToSlot` _save _returnvalue)))))))
    (:`then_1`
      (`KismetSystemLibrary.Delay` 0.1)
      (`/Engine/EditorBlueprintResources/StandardMacros.DoOnce` false
        (:`Completed`
          (`GameplayStatics.PlaySound2D` "/Game/Audio/Sounds/hurt3_Cue.hurt3_Cue" 1.0 1.0 0.0 null null)
          (`GameplayStatics.SaveGameToSlot` _save_2 _returnvalue_2)
          (`KismetSystemLibrary.Delay` 0.5)
          (`GameplayStatics.OpenLevel` "Lobby" false))))
    (:`then_2`
      (`Character.LaunchCharacter` _asplayer_acorn (0.0 0.0 5.0) true true))))

(fn `UserConstructionScript`)