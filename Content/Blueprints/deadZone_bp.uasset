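; Dead zone trigger volume that ends the run when the player acorn enters it, with its box sized by a Size variable in the construction script.
; On overlap it zeroes the game instance's seeds, calls LoseLife, and deletes all gadgets from both the player and its save.
; It also starts a game-over transition animation, whose finished callback opens the Lobby level.
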(event `self.Box.OnComponentBeginOverlap`
  (params (OverlappedComponent :type "PrimitiveComponent Object Reference") (OtherActor :type "Actor Object Reference") (OtherComp :type "PrimitiveComponent Object Reference") (OtherBodyIndex :type Integer) (bFromSweep :type Boolean) (SweepResult :type "HitResult Structure (by ref)"))
  (bind _asplayer_acorn (cast `/Game/Player/Player_Acorn` OtherActor))
  (bind _asacorn_game_instance (cast `/Game/Blueprints/acorn_gameInstance` (`GameplayStatics.GetGameInstance`)))
  (set `/Game/Blueprints/acorn_gameInstance.seeds` 0 _asacorn_game_instance)
  (bind (_anim1 _returnvalue) (`/Game/Blueprints/7646_fuctionLibrary.transitionGameOver` "Forward"))
  (`UserWidget.BindToAnimationFinished` _returnvalue _anim1 (delegate `onFinishTransition`))
  (`/Game/Player/Player_Acorn.loseLife` _asplayer_acorn)
  (`/Game/Blueprints/defaultSaveGame.deleteAllGadgets` (`/Game/Player/Player_Acorn.save` _asplayer_acorn))
  (`/Game/Player/Player_Acorn.deleteAllGadgets` _asplayer_acorn))

(event `onFinishTransition`
  (`GameplayStatics.OpenLevel` "Lobby"))

(fn `UserConstructionScript`
  (`BoxComponent.SetBoxExtent` (`self.Box`) (`self.size`) true))