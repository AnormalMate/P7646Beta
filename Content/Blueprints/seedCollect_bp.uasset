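; Collectible seed pickup for the Acorn player that adds to the seed count when touched.
; A fast looping timer keeps the actor rotated toward the player's follow camera, billboard-style.
; On sphere overlap by Player_Acorn it increments seeds on both the player and the game instance, plays a collect sound, and destroys itself.
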(event `self.ReceiveBeginPlay`
  (`KismetSystemLibrary.K2_SetTimerDelegate` (delegate `event1`) 0.01 true))

(event `event1`
  (bind _asplayer_acorn (cast `/Game/Player/Player_Acorn` (`GameplayStatics.GetPlayerCharacter` 0) :!pure true))
  (`/Engine/EditorBlueprintResources/StandardMacros.IsValid` _asplayer_acorn
    (:`Is Valid`
      (`self.K2_SetActorRotation` (`KismetMathLibrary.FindLookAtRotation` (`self.K2_GetActorLocation`) (`SceneComponent.K2_GetComponentLocation` (`/Game/Player/Player_Acorn.FollowCamera` _asplayer_acorn)))))))

(event `self.Sphere.OnComponentBeginOverlap`
  (params (OverlappedComponent :type "PrimitiveComponent Object Reference") (OtherActor :type "Actor Object Reference") (OtherComp :type "PrimitiveComponent Object Reference") (OtherBodyIndex :type Integer) (bFromSweep :type Boolean) (SweepResult :type "HitResult Structure (by ref)"))
  (bind _asplayer_acorn (cast `/Game/Player/Player_Acorn` OtherActor))
  (`/Engine/EditorBlueprintResources/StandardMacros.IncrementInt` (`/Game/Player/Player_Acorn.seeds` _asplayer_acorn)
    (:`  `
      (`GameplayStatics.PlaySound2D` "/Game/Audio/Sounds/seedCollect_Cue.seedCollect_Cue" 2.0 1.0 0.0 null null)
      (bind _asacorn_game_instance (cast `/Game/Blueprints/acorn_gameInstance` (`GameplayStatics.GetGameInstance`)))
      (set `/Game/Blueprints/acorn_gameInstance.seeds` (+ (`/Game/Blueprints/acorn_gameInstance.seeds` _asacorn_game_instance) 1) _asacorn_game_instance)
      (`self.K2_DestroyActor`))))

(fn `UserConstructionScript`)