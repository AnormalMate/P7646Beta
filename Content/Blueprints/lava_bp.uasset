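; Lava hazard actor with a Plane surface that melts the player acorn on contact.
; On BeginPlay it passes its Uv and Speed values to the plane's material parameters for UV and panner speed.
; When the plane is hit by a Player_Acorn, it spawns Acorn_melt_bp at the player's location and rotation, hides the player's mesh and plays a 2D hurt sound.
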(event `self.ReceiveBeginPlay`
  (`MeshComponent.SetScalarParameterValueOnMaterials` (`self.Plane`) "uv" (`self.uv`))
  (`MeshComponent.SetScalarParameterValueOnMaterials` (`self.Plane`) "pannerSpeed" (`self.speed`)))

(event `self.Plane.OnComponentHit`
  (params (HitComponent :type "PrimitiveComponent Object Reference") (OtherActor :type "Actor Object Reference") (OtherComp :type "PrimitiveComponent Object Reference") (NormalImpulse :type "Vector Structure") (Hit :type "HitResult Structure (by ref)"))
  (bind _asplayer_acorn (cast `/Game/Player/Player_Acorn` OtherActor))
  (bind (_returnvalue_location _returnvalue_rotation) (`KismetMathLibrary.BreakTransform` (`self.GetTransform` _asplayer_acorn)))
  (`|SpawnActorFromClass` "/Game/Blueprints/acorn_melt_bp.acorn_melt_bp_C" (`KismetMathLibrary.MakeTransform` _returnvalue_location _returnvalue_rotation) "AlwaysSpawn" "OverrideRootScale" null null)
  (`SceneComponent.SetVisibility` (`Character.Mesh` _asplayer_acorn) false false)
  (`GameplayStatics.PlaySound2D` "/Game/Audio/Sounds/hurt3_Cue.hurt3_Cue" 1.0 1.0 0.0 null null))

(fn `UserConstructionScript`)