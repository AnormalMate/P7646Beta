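; Blueprint function library of shared helpers for player lookup, animation playback and screen transitions.
; GetPlayer returns player 0's character cast to Player_Acorn, and PlayAnimationLength plays a non-looping animation on a skeletal mesh and returns its length.
; Both transition functions spawn a TransitionUI widget, play it in the given mode and return it with its animation.
; The game-over variant also swaps in its own image texture.
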(fn `getPlayer`
  (returns (`AsPlayer Acorn` :type "/Game/Player/Player_Acorn Object Reference"))
  (bind _asplayer_acorn (cast `/Game/Player/Player_Acorn` (`GameplayStatics.GetPlayerCharacter` null)))
  (return _asplayer_acorn))

(fn `playAnimationLength`
  (params (skeletalMesh :type "SkeletalMeshComponent Object Reference") (Anim :type "AnimSequenceBase Object Reference"))
  (returns (ReturnValue :type "Float (double-precision)"))
  (`SkeletalMeshComponent.PlayAnimation` skeletalMesh Anim false)
  (bind _returnvalue (`AnimSequenceBase.GetPlayLength` Anim))
  (return _returnvalue))

(fn `transition`
  (params (playMode :type "EUMGSequencePlayMode Enum" :default "Forward"))
  (returns (anim1 :type "WidgetAnimation Object Reference") (ReturnValue :type "/Game/UI/transitionUI Object Reference"))
  (bind _returnvalue (`|CreateWidget` "/Game/UI/transitionUI.transitionUI_C"))
  (`UserWidget.AddToPlayerScreen` _returnvalue 10)
  (`/Game/UI/transitionUI.playanim` _returnvalue playMode)
  (return (`/Game/UI/transitionUI.anim1` _returnvalue) _returnvalue))

(fn `transitionGameOver`
  (params (playMode :type "EUMGSequencePlayMode Enum" :default "Forward"))
  (returns (anim1 :type "WidgetAnimation Object Reference") (ReturnValue :type "/Game/UI/transitionUI Object Reference"))
  (bind _returnvalue (`|CreateWidget` "/Game/UI/transitionUI.transitionUI_C"))
  (`UserWidget.AddToPlayerScreen` _returnvalue 10)
  (`/Game/UI/transitionUI.playanim` _returnvalue playMode)
  (`Image.SetBrushFromTexture` (`/Game/UI/transitionUI.Image_12` _returnvalue) "/Game/UI/transitionGameOver.transitionGameOver" true)
  (return (`/Game/UI/transitionUI.anim1` _returnvalue) _returnvalue))