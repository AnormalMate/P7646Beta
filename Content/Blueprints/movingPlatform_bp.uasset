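; Moving platform Blueprint that slides its Cube vertically or sideways, started at BeginPlay or, with MoveWhenHit, by a Player_Acorn hit.
; An optional Switch, polled by a 0.1-second looping timer, gates movement.
; DoOnce-guarded MoveComponentTo chains handle delayed out-and-back trips with optional looping, or snap the Cube back with collision briefly disabled.
; PlatformMoveCue plays on movement; Tick stops it when actor velocity is zero.
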(event `event1`
  (bind _cube (`self.Cube`))
  (bind _switch (`self.switch`))
  (bind _delayafterswitch (`self.delayAfterSwitch`))
  (bind _platformmove_cue (`self.platformMove_Cue`))
  (bind (_relativelocation_x _relativelocation_y _relativelocation_z) (`KismetMathLibrary.BreakVector` (`SceneComponent.RelativeLocation` _cube)))
  (bind (_relativelocation_x_2 _relativelocation_y_2 _relativelocation_z_2) (`KismetMathLibrary.BreakVector` (`SceneComponent.RelativeLocation` _cube)))
  (bind (_relativelocation_x_3 _relativelocation_y_3) (`KismetMathLibrary.BreakVector` (`SceneComponent.RelativeLocation` _cube)))
  (bind (_relativelocation_x_4 _relativelocation_y_4) (`KismetMathLibrary.BreakVector` (`SceneComponent.RelativeLocation` _cube)))
  (bind (_relativelocation_x_5 _relativelocation_y_5) (`KismetMathLibrary.BreakVector` (`SceneComponent.RelativeLocation` _cube)))
  (bind (_relativelocation_x_6 _relativelocation_y_6) (`KismetMathLibrary.BreakVector` (`SceneComponent.RelativeLocation` _cube)))
  (`/Engine/EditorBlueprintResources/StandardMacros.IsValid` (`self.switch`)
    (:`Is Valid`
      (switch `/Game/Enums/EMovingPlatformType` (`self.movementType`) :!label _label
        (:`NewEnumerator0`
          (`AudioComponent.Play` _platformmove_cue 0.0)
          (`/Engine/EditorBlueprintResources/StandardMacros.IsValid` _switch :!label _label_2
            (:`Is Valid`
              (if (`/Game/Blueprints/switchBaseActor.isOn` (`self.switch`))
                (`KismetSystemLibrary.Delay` _delayafterswitch)
                (`/Engine/EditorBlueprintResources/StandardMacros.DoOnce` false :!label _label_3
                  (:`Completed`
                    (`KismetSystemLibrary.MoveComponentTo` _cube (`KismetMathLibrary.MakeVector` _relativelocation_x_3 _relativelocation_y_3 (`self.upLoc`)) (`SceneComponent.RelativeRotation` _cube) false false (`self.moveSpeed`))
                    (if (`self.disappearWhenFinishMove`)
                      (`KismetSystemLibrary.Delay` 1.0)
                      (`PrimitiveComponent.SetCollisionEnabled` _cube "NoCollision")
                      (`KismetSystemLibrary.Delay` 0.1)
                      (`SceneComponent.K2_SetRelativeLocation` _cube (`KismetMathLibrary.MakeVector` _relativelocation_x_4 _relativelocation_y_4) false false)
                      (`PrimitiveComponent.SetCollisionEnabled` _cube "QueryAndPhysics")
                      (`AudioComponent.Stop` (`self.platformMove_Cue`) :!label _label_4)
                      (else
                        (`/Engine/EditorBlueprintResources/StandardMacros.DoOnce` false :!label _label_5
                          (:`Completed`
                            (`KismetSystemLibrary.Delay` (`self.delayBeforeLoop`))
                            (`KismetSystemLibrary.MoveComponentTo` _cube (`KismetMathLibrary.MakeVector` _relativelocation_x_5 _relativelocation_y_5) (`SceneComponent.RelativeRotation` _cube) false false (`self.moveSpeed`))
                            (`KismetSystemLibrary.Delay` (`self.delayBeforeLoop`))
                            (if (`self.loop`)
                              (`|ExecutionSequence`
                                (:`then_0`
                                  (goto _label_2))
                                (:`then_1`
                                  (goto _label_3 :!via `Reset`))
                                (:`then_2`
                                  (goto _label_5 :!via `Reset`))
                                (:`then_3`
                                  (`KismetSystemLibrary.Delay` 0.1)
                                  (goto _label_3))))))))))
                (else
                  (goto _label_5))))
            (:`Is Not Valid`
              (goto _label_3))))
        (:`NewEnumerator1`
          (`AudioComponent.Play` _platformmove_cue 0.0)
          (`/Engine/EditorBlueprintResources/StandardMacros.IsValid` _switch :!label _label_6
            (:`Is Valid`
              (if (`/Game/Blueprints/switchBaseActor.isOn` (`self.switch`))
                (`KismetSystemLibrary.Delay` _delayafterswitch)
                (`/Engine/EditorBlueprintResources/StandardMacros.DoOnce` false :!label _label_7
                  (:`Completed`
                    (`KismetSystemLibrary.MoveComponentTo` _cube (`KismetMathLibrary.MakeVector` (`self.rightLoc`) _relativelocation_y_2 _relativelocation_z_2) (`SceneComponent.RelativeRotation` _cube) false false (`self.moveSpeed`))
                    (if (`self.disappearWhenFinishMove`)
                      (`KismetSystemLibrary.Delay` 1.0)
                      (`PrimitiveComponent.SetCollisionEnabled` _cube "NoCollision")
                      (`SceneComponent.K2_SetRelativeLocation` _cube (`KismetMathLibrary.MakeVector` _relativelocation_x_6 _relativelocation_y_6) false false)
                      (`KismetSystemLibrary.Delay` 0.1)
                      (`PrimitiveComponent.SetCollisionEnabled` _cube "QueryAndPhysics")
                      (goto _label_4)
                      (else
                        (`/Engine/EditorBlueprintResources/StandardMacros.DoOnce` false :!label _label_8
                          (:`Completed`
                            (`KismetSystemLibrary.Delay` (`self.delayBeforeLoop`))
                            (`KismetSystemLibrary.MoveComponentTo` _cube (`KismetMathLibrary.MakeVector` 0.0 _relativelocation_y _relativelocation_z) (`SceneComponent.RelativeRotation` _cube) false false (`self.moveSpeed`))
                            (`KismetSystemLibrary.Delay` (`self.delayBeforeLoop`))
                            (`|ExecutionSequence`
                              (:`then_0`
                                (goto _label_7 :!via `Reset`))
                              (:`then_1`
                                _)
                              (:`then_2`
                                (goto _label_8 :!via `Reset`))
                              (:`then_3`
                                (`KismetSystemLibrary.Delay` 0.1)
                                (goto _label_7)))))))))
                (else
                  (goto _label_8))))
            (:`Is Not Valid`
              (goto _label_7)))
          (if (`self.loop`)
            (goto _label_6)))))))

(event `self.ReceiveBeginPlay`
  (`parent.ReceiveBeginPlay`)
  (`|ExecutionSequence`
    (:`then_0`
      (if (not (`self.moveWhenHit`))
        (goto _label)))
    (:`then_1`
      (`KismetSystemLibrary.K2_SetTimerDelegate` (delegate `event1`) 0.1 true))))

(event `self.Cube.OnComponentHit`
  (params (HitComponent :type "PrimitiveComponent Object Reference") (OtherActor :type "Actor Object Reference") (OtherComp :type "PrimitiveComponent Object Reference") (NormalImpulse :type "Vector Structure") (Hit :type "HitResult Structure (by ref)"))
  (cast `/Game/Player/Player_Acorn` OtherActor)
  (if (`self.moveWhenHit`)
    (goto _label)))

(event `self.ReceiveTick`
  (params (DeltaSeconds :type "Float (single-precision)"))
  (if (<= (`KismetMathLibrary.VSize` (`self.GetVelocity`)) 0.0)
    (`/Engine/EditorBlueprintResources/StandardMacros.DoOnce` false :!label _label_9
      (:`Completed`
        (`AudioComponent.Stop` (`self.platformMove_Cue`))))
    (else
      (goto _label_9 :!via `Reset`))))

(fn `UserConstructionScript`
  (`parent.UserConstructionScript`))