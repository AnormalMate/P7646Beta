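; Red apple enemy character that wanders the navmesh, chases the player and attacks up close.
; Tick polls the SightRange and Attack overlaps to start chasing or attacking; losing sight resumes wandering after a delay.
; Attacks are DoOnce-gated, draining player health, launching them back and playing an attack animation.
; Punch counts down hits with knockback and a brief stun, then plays death and destroys the actor.
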(event `wander`
  (if (not (`self.chase`))
    (`|AIMoveTo` self (`NavigationSystemV1.K2_GetRandomLocationInNavigableRadius` (`self.K2_GetActorLocation`) 1000.0 null null) null
      (:`OnSuccess`
        _)
      (:`OnFail`
        _))
    (`self.wander`)))

(event `self.ReceiveBeginPlay`
  (`self.wander`))

(event `chasePlayer`
  (bind _asplayer_acorn (`/Game/Blueprints/7646_fuctionLibrary.getPlayer`))
  (if (not (`/Game/Player/Player_Acorn.dead?` _asplayer_acorn))
    (set `self.chase` true)
    (`|AIMoveTo` self (`self.K2_GetActorLocation` (`GameplayStatics.GetPlayerCharacter` 0)) null 10.0 true
      (:`OnFail`
        (`KismetSystemLibrary.Delay` 3.0 :!label _label)
        (set `self.chase` false)
        (`self.wander`)))))

(event `self.sightRange.OnComponentBeginOverlap`
  (params (OverlappedComponent :type "PrimitiveComponent Object Reference") (OtherActor :type "Actor Object Reference") (OtherComp :type "PrimitiveComponent Object Reference") (OtherBodyIndex :type Integer) (bFromSweep :type Boolean) (SweepResult :type "HitResult Structure (by ref)"))
  (bind _asplayer_acorn (cast `/Game/Player/Player_Acorn` OtherActor))
  (if (`/Game/Player/Player_Acorn.dead?` _asplayer_acorn)
    _))

(event `self.ReceiveTick`
  (params (DeltaSeconds :type "Float (single-precision)"))
  (bind _mesh (`self.Mesh`))
  (`|ExecutionSequence`
    (:`then_0`
      (if (`PrimitiveComponent.IsOverlappingActor` (`self.sightRange`) (`GameplayStatics.GetPlayerCharacter` 0))
        (`self.chasePlayer`)))
    (:`then_1`
      (if (`PrimitiveComponent.IsOverlappingActor` (`self.attack`) (`GameplayStatics.GetPlayerCharacter` 0))
        (`KismetSystemLibrary.Delay` 0.2)
        (`/Engine/EditorBlueprintResources/StandardMacros.DoOnce` false :!label _label_2
          (:`Completed`
            (set `self.canAttack?` true)
            (bind _asplayer_acorn (`/Game/Blueprints/7646_fuctionLibrary.getPlayer`))
            (if (`/Game/Player/Player_Acorn.dead?` _asplayer_acorn)
              (`self.wander`)
              (elif (`self.canAttack?`)
                (if (not (`self.dead`))
                  (set `self.canAttack?` false)
                  (set `/Game/Player/Player_Acorn.enemyAttacked` true _asplayer_acorn)
                  (set `/Game/Player/Player_Acorn.Health` (- (`/Game/Player/Player_Acorn.Health` _asplayer_acorn) 0.2) _asplayer_acorn)
                  (`GameplayStatics.PlaySound2D` "/Game/Audio/Sounds/hurt3_Cue.hurt3_Cue" 1.0 1.0 0.0 null null)
                  (bind (_returnvalue_x _returnvalue_y) (`KismetMathLibrary.BreakVector` (* (`self.GetActorForwardVector` _asplayer_acorn) -500)))
                  (`self.LaunchCharacter` _asplayer_acorn (`KismetMathLibrary.MakeVector` _returnvalue_x _returnvalue_y 500.0) true true)
                  (if (not (`self.dead`))
                    (set `/Game/Player/Player_Acorn.enemyAttacked` false _asplayer_acorn)
                    (`GameplayStatics.PlaySoundAtLocation` "/Game/Audio/Sounds/punch_1_Cue.punch_1_Cue" (`self.K2_GetActorLocation`) (struct) 1.0 1.0 0.0 null null null)
                    (bind _returnvalue (`/Game/Blueprints/7646_fuctionLibrary.playAnimationLength` _mesh "/Game/Character/RedApple_anims_Armature_attack.RedApple_anims_Armature_attack"))
                    (`KismetSystemLibrary.Delay` _returnvalue)
                    (`SkeletalMeshComponent.PlayAnimation` _mesh "/Game/Character/RedApple_anims_Armature_walk.RedApple_anims_Armature_walk" true)
                    (`self.chasePlayer`)
                    (`KismetSystemLibrary.Delay` 1.0)
                    (set `self.canAttack?` true)
                    (goto _label_2 :!via `Reset`)))))))))))

(event `self.sightRange.OnComponentEndOverlap`
  (params (OverlappedComponent :type "PrimitiveComponent Object Reference") (OtherActor :type "Actor Object Reference") (OtherComp :type "PrimitiveComponent Object Reference") (OtherBodyIndex :type Integer))
  (cast `/Game/Player/Player_Acorn` OtherActor)
  (goto _label))

(event `self.attack.OnComponentEndOverlap`
  (params (OverlappedComponent :type "PrimitiveComponent Object Reference") (OtherActor :type "Actor Object Reference") (OtherComp :type "PrimitiveComponent Object Reference") (OtherBodyIndex :type Integer))
  (bind _asplayer_acorn (cast `/Game/Player/Player_Acorn` OtherActor))
  (set `self.canAttack?` false)
  (set `/Game/Player/Player_Acorn.enemyAttacked` false _asplayer_acorn))

(event `/Game/Blueprints/7646_blueprintInterface.punch`
  (bind _charactermovement (`self.CharacterMovement`))
  (bind (_returnvalue_x _returnvalue_y) (`KismetMathLibrary.BreakVector` (* (`self.GetActorForwardVector`) -500.0)))
  (if (<= (`self.hits`) 0)
    (`/Engine/EditorBlueprintResources/StandardMacros.DoOnce` false
      (:`Completed`
        (bind _asplayer_acorn (`/Game/Blueprints/7646_fuctionLibrary.getPlayer`))
        (set `self.canAttack?` false)
        (bind (_returnvalue_x_2 _returnvalue_y_2) (`KismetMathLibrary.BreakVector` (* (`self.GetActorForwardVector` _asplayer_acorn) 500.0)))
        (`self.LaunchCharacter` (`KismetMathLibrary.MakeVector` _returnvalue_x_2 _returnvalue_y_2 500.0) true true)
        (`GameplayStatics.SpawnSoundAtLocation` "/Game/Audio/Sounds/appleMan/appledie_Cue.appledie_Cue" (`self.K2_GetActorLocation`) (struct) 1.0 1.0 0.0 null null)
        (set `self.dead` true)
        (`CharacterMovementComponent.SetMovementMode` (`self.CharacterMovement`) "MOVE_None" 0)
        (bind _returnvalue (`/Game/Blueprints/7646_fuctionLibrary.playAnimationLength` (`self.Mesh`) "/Game/Character/RedApple_anims_Armature_die.RedApple_anims_Armature_die"))
        (`KismetSystemLibrary.Delay` _returnvalue)
        (`KismetSystemLibrary.Delay` 1.0)
        (`self.K2_DestroyActor`)))
    (else
      (`/Engine/EditorBlueprintResources/StandardMacros.DecrementInt` (`self.hits`)
        (:`  `
          (`GameplayStatics.SpawnSoundAtLocation` "/Game/Audio/Sounds/appleMan/applehurt_Cue.applehurt_Cue" (`self.K2_GetActorLocation`) (struct) 1.0 1.0 0.0 null null)
          (`CharacterMovementComponent.SetMovementMode` _charactermovement "MOVE_None" 0)
          (set `self.canAttack?` false)
          (`self.LaunchCharacter` (`KismetMathLibrary.MakeVector` _returnvalue_x _returnvalue_y 100.0) true true)
          (`KismetSystemLibrary.Delay` 1.0)
          (`CharacterMovementComponent.SetMovementMode` _charactermovement "MOVE_Walking" 0)
          (set `self.canAttack?` true))))))

(fn `UserConstructionScript`)