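; Trigger volume that swaps the visible scene and fog look as the Player_Acorn passes through it.
; Scene2 starts hidden on BeginPlay, and each time the player leaves the Box a FlipFlop alternates visibility between Scene1 and Scene2.
; The same toggle applies one of two fog color and density sets, unhiding the Fog actor on the first state only if SetFogHidden is true.
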(event `self.ReceiveBeginPlay`
  (bind _scene2 (`self.scene2`))
  (`/Engine/EditorBlueprintResources/StandardMacros.IsValid` _scene2
    (:`Is Valid`
      (`self.SetActorHiddenInGame` _scene2 true))))

(event `self.Box.OnComponentEndOverlap`
  (params (OverlappedComponent :type "PrimitiveComponent Object Reference") (OtherActor :type "Actor Object Reference") (OtherComp :type "PrimitiveComponent Object Reference") (OtherBodyIndex :type Integer))
  (bind _scene1 (`self.scene1`))
  (bind _fog (`self.fog`))
  (bind _scene2 (`self.scene2`))
  (bind _fog_2 (`self.fog`))
  (bind _exponentialheightfog (`/Game/Blueprints/fog_bp.ExponentialHeightFog` _fog))
  (bind _exponentialheightfog_2 (`/Game/Blueprints/fog_bp.ExponentialHeightFog` _fog_2))
  (cast `/Game/Player/Player_Acorn` OtherActor)
  (`/Engine/EditorBlueprintResources/StandardMacros.FlipFlop`
    (:`A`
      (`/Engine/EditorBlueprintResources/StandardMacros.IsValid` _scene1
        (:`Is Valid`
          (`self.SetActorHiddenInGame` _scene1 true)
          (`self.SetActorHiddenInGame` (`self.scene2`) false))
        (:`Is Not Valid`
          _))
      (`/Engine/EditorBlueprintResources/StandardMacros.IsValid` _fog
        (:`Is Valid`
          (if (`self.setFogHidden`)
            (`self.SetActorHiddenInGame` _fog false))
          (`ExponentialHeightFogComponent.SetFogInscatteringColor` _exponentialheightfog (`self.fogColor1`))
          (`ExponentialHeightFogComponent.SetFogDensity` _exponentialheightfog (`self.fog1Density`)))))
    (:`B`
      (`/Engine/EditorBlueprintResources/StandardMacros.IsValid` _scene2
        (:`Is Valid`
          (`self.SetActorHiddenInGame` (`self.scene1`) false)
          (`self.SetActorHiddenInGame` _scene2 true))
        (:`Is Not Valid`
          _))
      (`/Engine/EditorBlueprintResources/StandardMacros.IsValid` _fog_2
        (:`Is Valid`
          (`self.SetActorHiddenInGame` _fog_2 false)
          (`ExponentialHeightFogComponent.SetFogInscatteringColor` _exponentialheightfog_2 (`self.fogColor2`))
          (`ExponentialHeightFogComponent.SetFogDensity` _exponentialheightfog_2 (`self.fog2Density`)))))))

(fn `UserConstructionScript`)