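; Grenade maniac enemy, a kamikaze character that leaps and blows itself up when the player gets close.
; It moves to one random navigable point on BeginPlay, then Tick checks two overlap volumes against the player.
; Inside SightRange it chases if CanChase allows.
; Inside AttackRange a resettable DoOnce launches it forward and upward, then a second later spawns GrenadeSeedsBox_bp, plays an explosion sound and destroys itself.
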(event `wander`
  (`|AIMoveTo` self (`NavigationSystemV1.K2_GetRandomLocationInNavigableRadius` (`self.K2_GetActorLocation`) 1000.0 null null) null))

(event `self.ReceiveBeginPlay`
  (`parent.ReceiveBeginPlay`)
  (`self.wander`))

(event `self.ReceiveTick`
  (params (DeltaSeconds :type "Float (single-precision)"))
  (bind (_returnvalue_x _returnvalue_y) (`KismetMathLibrary.BreakVector` (* (`self.GetActorForwardVector`) 500)))
  (`parent.ReceiveTick` DeltaSeconds)
  (`|ExecutionSequence`
    (:`then_0`
      (if (`PrimitiveComponent.IsOverlappingActor` (`self.sightRange`) (`GameplayStatics.GetPlayerCharacter` 0))
        (if (`self.canChase`)
          (`|AIMoveTo` self (0.0 0.0 0.0) (`GameplayStatics.GetPlayerCharacter` 0)
            (:`then`
              (set `self.chasing` true))))
        (else
          (set `self.chasing` false))))
    (:`then_1`
      (if (`PrimitiveComponent.IsOverlappingActor` (`self.attackRange`) (`GameplayStatics.GetPlayerCharacter` 0))
        (`/Engine/EditorBlueprintResources/StandardMacros.DoOnce` false :!label _label
          (:`Completed`
            (`self.LaunchCharacter` (`KismetMathLibrary.MakeVector` _returnvalue_x _returnvalue_y 1000.0) true true)
            (`KismetSystemLibrary.Delay` 1.0)
            (`|SpawnActorFromClass` "/Game/Blueprints/grenadeSeedsBox_bp.grenadeSeedsBox_bp_C" (`self.GetTransform`) "AlwaysSpawn" "OverrideRootScale" null null)
            (`GameplayStatics.PlaySoundAtLocation` "/Game/Audio/Sounds/Explosion_Cue.Explosion_Cue" (`self.K2_GetActorLocation`) (struct) 5.0 1.0 0.0 null null null)
            (`self.K2_DestroyActor`)))
        (else
          (goto _label :!via `Reset`))))))

(fn `UserConstructionScript`
  (`parent.UserConstructionScript`))