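; Blueprint actor that plays a short acorn melt transition before restarting the level.
; On BeginPlay it switches the player's view to the owner of its Camera component and sinks its StaticMesh downward over two seconds.
; After a brief delay it casts the game mode to 7646GameMode and calls ResetLevel, which fires before the sinking move finishes.
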(event `self.ReceiveBeginPlay`
  (bind _staticmesh (`self.StaticMesh`))
  (`PlayerController.SetViewTargetWithBlend` (`GameplayStatics.GetPlayerController` 0) (`ActorComponent.GetOwner` (`self.camera`)) 0.0 "VTBlend_Linear" 0.0 false)
  (`KismetSystemLibrary.MoveComponentTo` _staticmesh (0.0 0.0 -500.0) (`SceneComponent.RelativeRotation` _staticmesh) false false 2.0)
  (`KismetSystemLibrary.Delay` 0.5)
  (bind _as7646game_mode (cast `/Game/Player/7646GameMode` (`GameplayStatics.GetGameMode`)))
  (`GameModeBase.ResetLevel` _as7646game_mode))

(fn `UserConstructionScript`)