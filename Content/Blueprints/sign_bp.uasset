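; Sign actor that shows its text on screen when the Punch event fires while Player_Acorn is within its Box trigger.
; Box overlap opens and closes a Gate, and a DoOnce behind it limits Punch to creating one TextSign_ui widget, which receives the sign's Text.
; Leaving the box removes the widget and resets the DoOnce so the sign can be read again.
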(event `/Game/Blueprints/7646_blueprintInterface.punch`
  (`/Engine/EditorBlueprintResources/StandardMacros.Gate` true :!label _label
    (:`Exit`
      (`/Engine/EditorBlueprintResources/StandardMacros.DoOnce` false :!label _label_2
        (:`Completed`
          (bind _returnvalue (`|CreateWidget` "/Game/UI/textSign_ui.textSign_ui_C" null "(placeholder)"))
          (bind _output_get (set `self.ui1` _returnvalue))
          (`UserWidget.AddToPlayerScreen` _output_get 0)
          (set `/Game/UI/textSign_ui.text` (`self.text`) (`self.ui1`)))))))

(event `self.Box.OnComponentBeginOverlap`
  (params (OverlappedComponent :type "PrimitiveComponent Object Reference") (OtherActor :type "Actor Object Reference") (OtherComp :type "PrimitiveComponent Object Reference") (OtherBodyIndex :type Integer) (bFromSweep :type Boolean) (SweepResult :type "HitResult Structure (by ref)"))
  (cast `/Game/Player/Player_Acorn` OtherActor)
  (goto _label :!via `Open`))

(event `self.Box.OnComponentEndOverlap`
  (params (OverlappedComponent :type "PrimitiveComponent Object Reference") (OtherActor :type "Actor Object Reference") (OtherComp :type "PrimitiveComponent Object Reference") (OtherBodyIndex :type Integer))
  (bind _ui1 (`self.ui1`))
  (cast `/Game/Player/Player_Acorn` OtherActor)
  (`/Engine/EditorBlueprintResources/StandardMacros.IsValid` _ui1
    (:`Is Valid`
      (`Widget.RemoveFromParent` _ui1)
      (`|ExecutionSequence`
        (:`then_0`
          (goto _label_2 :!via `Reset`))
        (:`then_1`
          (goto _label :!via `Close`))))
    (:`Is Not Valid`
      (goto _label :!via `Close`))))

(fn `UserConstructionScript`)