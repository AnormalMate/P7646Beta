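; An invisible box actor whose Cube mesh appears and becomes solid only while a referenced Switch is on.
; BeginPlay hides the Cube with collision disabled and starts a looping 0.01-second timer that polls the Switch's IsOn state.
; When on, the Cube is visible with query and physics collision; when off or the Switch is invalid, it returns to hidden and non-colliding.
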(event `self.ReceiveBeginPlay`
  (bind _cube (`self.Cube`))
  (`KismetSystemLibrary.K2_SetTimerDelegate` (delegate `event1`) 0.01 true)
  (`SceneComponent.SetVisibility` _cube false false :!label _label)
  (`PrimitiveComponent.SetCollisionEnabled` _cube "NoCollision"))

(event `event1`
  (bind _switch (`self.switch`))
  (bind _cube (`self.Cube`))
  (`/Engine/EditorBlueprintResources/StandardMacros.IsValid` _switch
    (:`Is Valid`
      (if (`/Game/Blueprints/switchBaseActor.isOn` _switch)
        (`SceneComponent.SetVisibility` _cube true false)
        (`PrimitiveComponent.SetCollisionEnabled` _cube "QueryAndPhysics")
        (else
          (goto _label))))
    (:`Is Not Valid`
      (goto _label))))

(fn `UserConstructionScript`)