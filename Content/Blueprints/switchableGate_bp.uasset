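; A gate Blueprint whose Cube disappears and stops blocking while its linked Switch is on.
; A looping timer started at BeginPlay polls the Switch's IsOn state, toggling the Cube's visibility and collision to match, rather than reacting to a switch event.
; The construction script passes the Uv variable to the Cube's materials as the "UV" scalar parameter.
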(event `self.ReceiveBeginPlay`
  (`KismetSystemLibrary.K2_SetTimerDelegate` (delegate `event1`) 0.01 true))

(event `event1`
  (bind _switch (`self.switch`))
  (bind _cube (`self.Cube`))
  (`/Engine/EditorBlueprintResources/StandardMacros.IsValid` _switch
    (:`Is Valid`
      (if (`/Game/Blueprints/switchBaseActor.isOn` _switch)
        (`SceneComponent.SetVisibility` _cube false false)
        (`PrimitiveComponent.SetCollisionEnabled` _cube "NoCollision")
        (else
          (`SceneComponent.SetVisibility` _cube true false)
          (`PrimitiveComponent.SetCollisionEnabled` _cube "QueryAndPhysics"))))))

(fn `UserConstructionScript`
  (`MeshComponent.SetScalarParameterValueOnMaterials` (`self.Cube`) "UV" (`self.uv`)))