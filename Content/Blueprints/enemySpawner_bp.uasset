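; Trigger-area spawner that creates an enemy of EnemyClass when Player_Acorn enters SpawnArea.
; The enemy appears at SpawnLoc, adjusted to avoid collisions if possible, and its reference is stored.
; A DoOnce blocks repeat spawns, resetting only when the player leaves the area after that enemy is no longer valid, so re-entry spawns a replacement.
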(event `self.spawnArea.OnComponentBeginOverlap`
  (params (OverlappedComponent :type "PrimitiveComponent Object Reference") (OtherActor :type "Actor Object Reference") (OtherComp :type "PrimitiveComponent Object Reference") (OtherBodyIndex :type Integer) (bFromSweep :type Boolean) (SweepResult :type "HitResult Structure (by ref)"))
  (cast `/Game/Player/Player_Acorn` OtherActor)
  (`/Engine/EditorBlueprintResources/StandardMacros.DoOnce` false :!label _label
    (:`Completed`
      (bind _returnvalue (`|SpawnActorFromClass` (`self.enemyClass`) (`KismetMathLibrary.MakeTransform` (`SceneComponent.K2_GetComponentLocation` (`self.spawnLoc`))) "AdjustIfPossibleButAlwaysSpawn" "OverrideRootScale" null null))
      (set `self.Actor` _returnvalue))))

(event `self.spawnArea.OnComponentEndOverlap`
  (params (OverlappedComponent :type "PrimitiveComponent Object Reference") (OtherActor :type "Actor Object Reference") (OtherComp :type "PrimitiveComponent Object Reference") (OtherBodyIndex :type Integer))
  (cast `/Game/Player/Player_Acorn` OtherActor)
  (`/Engine/EditorBlueprintResources/StandardMacros.IsValid` (`self.Actor`)
    (:`Is Not Valid`
      (set `self.Actor` null)
      (goto _label :!via `Reset`))))

(fn `UserConstructionScript`)