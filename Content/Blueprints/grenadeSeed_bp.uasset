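; Homing seed projectile (grenadeSeed) that chases the player and damages Player_Acorn on contact.
; Each tick it turns to face player 0 and accelerates its Collision component along the Arrow's forward vector.
; Sphere overlap with the acorn sets Launched, applies a tiny upward launch that overrides horizontal velocity, reduces Health and destroys the seed.
; It also destroys itself on high-speed hits or after a random lifetime.
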(event `self.ReceiveTick`
  (params (DeltaSeconds :type "Float (single-precision)"))
  (`|ExecutionSequence`
    (:`then_1`
      (`self.K2_SetActorRotation` (`KismetMathLibrary.FindLookAtRotation` (`self.K2_GetActorLocation`) (`self.K2_GetActorLocation` (`GameplayStatics.GetPlayerCharacter` 0))))
      (`PrimitiveComponent.AddForce` (`self.collision`) (* (`SceneComponent.GetForwardVector` (`self.Arrow`)) 1200) "None" true))))

(event `self.ReceiveBeginPlay`
  (`KismetSystemLibrary.Delay` (`KismetMathLibrary.RandomFloatInRange` 7.0 15.0))
  (`self.K2_DestroyActor`))

(event `self.Sphere.OnComponentBeginOverlap`
  (params (OverlappedComponent :type "PrimitiveComponent Object Reference") (OtherActor :type "Actor Object Reference") (OtherComp :type "PrimitiveComponent Object Reference") (OtherBodyIndex :type Integer) (bFromSweep :type Boolean) (SweepResult :type "HitResult Structure (by ref)"))
  (bind _asplayer_acorn (cast `/Game/Player/Player_Acorn` OtherActor))
  (set `/Game/Player/Player_Acorn.launched` true _asplayer_acorn)
  (`Character.LaunchCharacter` _asplayer_acorn (0.0 0.0 5.0) true true)
  (set `/Game/Player/Player_Acorn.Health` (- (`/Game/Player/Player_Acorn.Health` _asplayer_acorn) 0.1) _asplayer_acorn)
  (`self.K2_DestroyActor`))

(event `self.ReceiveHit`
  (params (MyComp :type "PrimitiveComponent Object Reference") (Other :type "Actor Object Reference") (OtherComp :type "PrimitiveComponent Object Reference") (bSelfMoved :type Boolean) (HitLocation :type "Vector Structure") (HitNormal :type "Vector Structure") (NormalImpulse :type "Vector Structure") (Hit :type "HitResult Structure (by ref)"))
  (if (>= (`KismetMathLibrary.VSize` (`self.GetVelocity`)) 1000.0)
    (`self.K2_DestroyActor`)))

(fn `UserConstructionScript`)